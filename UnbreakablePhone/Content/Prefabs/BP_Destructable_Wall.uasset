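; Destructible wall Blueprint that spreads destruction to neighboring walls of the same class before removing itself.
; Its destroy event sets an IsDestroyed flag, then sphere-traces around the wall mesh and triggers the same event on nearby intact walls.
; The flag stops walls re-triggering each other in this recursive chain reaction, and each wall destroys its actor after a short delay.
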(event `Destroy wall`
  (bind _returnvalue (`SceneComponent.K2_GetComponentLocation` (`self.Destructible_Wall4x4`)))
  (set `self.isDestroyed` true)
  (bind _outhits (`KismetSystemLibrary.SphereTraceMultiForObjects` :`Start` _returnvalue :`End` _returnvalue :`Radius` 400.0 :`ObjectTypes` (`|MakeArray` (`self.Object Types`)) :`DrawTime` 1.0))
  (for _array_element _outhits
    (bind _asbp_destructable_wall (cast `/Game/Prefabs/BP_Destructable_Wall` (`.HitActor` (`GameplayStatics.BreakHitResult` _array_element))))
    (if (not (`/Game/Prefabs/BP_Destructable_Wall.isDestroyed` _asbp_destructable_wall))
      (`self.Destroy wall` _asbp_destructable_wall)))
  (`KismetSystemLibrary.Delay` 5.0)
  (`self.K2_DestroyActor`))

(fn `UserConstructionScript`)