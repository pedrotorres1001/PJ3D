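; BP_Painting_Stun is an interactable painting pickup that grants the player the stun ability.
; A sphere overlap with BP_Player enables input on the actor, adds an outline overlay material and shows a widget; leaving reverses all three.
; Pressing E while input is enabled sets HasStun on the player pawn, plays a power-up sound and destroys the painting.
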(event `Key|E`
  (params (Key :type "Key Structure"))
  (:`Pressed`
    (bind _asbp_player (cast `/Game/DamageSystem/Player/BP_Player` (`GameplayStatics.GetPlayerPawn` 0)))
    (set `/Game/DamageSystem/Player/BP_Player.HasStun` true _asbp_player)
    (`GameplayStatics.PlaySound2D` "/Game/Sounds/powerup.powerup" 1.0 1.0 0.0 null null)
    (`self.K2_DestroyActor`)))

(event `self.Sphere.OnComponentBeginOverlap`
  (params (OverlappedComponent :type "PrimitiveComponent Object Reference") (OtherActor :type "Actor Object Reference") (OtherComp :type "PrimitiveComponent Object Reference") (OtherBodyIndex :type Integer) (bFromSweep :type Boolean) (SweepResult :type "HitResult Structure (by ref)"))
  (cast `/Game/DamageSystem/Player/BP_Player` OtherActor)
  (`self.EnableInput` (`GameplayStatics.GetPlayerController` 0))
  (`MeshComponent.SetOverlayMaterial` (`self.StaticMeshComponent`) "/Game/Materials/Outline1.Outline1")
  (`SceneComponent.SetVisibility` (`self.widget_0`) true false))

(event `self.Sphere.OnComponentEndOverlap`
  (params (OverlappedComponent :type "PrimitiveComponent Object Reference") (OtherActor :type "Actor Object Reference") (OtherComp :type "PrimitiveComponent Object Reference") (OtherBodyIndex :type Integer))
  (cast `/Game/DamageSystem/Player/BP_Player` OtherActor)
  (`self.DisableInput` (`GameplayStatics.GetPlayerController` 0))
  (`MeshComponent.SetOverlayMaterial` (`self.StaticMeshComponent`) null)
  (`SceneComponent.SetVisibility` (`self.widget_0`) false false))

(fn `UserConstructionScript`)