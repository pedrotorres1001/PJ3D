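; TetrisPiece is a falling-block attack that hovers 200 units above its Target for one second, then slams down.
; The drop enables Cube physics with a downward impulse and sets a BP_Enemy target's capsule to ignore all channels.
; Hitting a BP_Enemy, BP_Enemy2 or BP_DroneBase adds another downward push, plays sound and sparks, and deals damage.
; It then ignores Pawn collision and destroys itself after a short delay.
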(event `self.ReceiveBeginPlay`
  (bind _cube (`self.Cube`))
  (`KismetSystemLibrary.Delay` 1.0)
  (set `self.Drop` true)
  (`PrimitiveComponent.SetSimulatePhysics` _cube true)
  (`PrimitiveComponent.AddImpulse` _cube (`KismetMathLibrary.MakeVector` 0.0 0.0 -1000.0) "None" true)
  (bind _asbp_enemy (cast `/Game/DamageSystem/Enemy/BP_Enemy` (`self.Target`)))
  (`PrimitiveComponent.SetCollisionResponseToAllChannels` (`Character.CapsuleComponent` _asbp_enemy) "ECR_Ignore"))

(event `self.ReceiveTick`
  (params (DeltaSeconds :type "Float (single-precision)"))
  (if (not (`self.Drop`))
    (`self.K2_SetActorLocation` (+ (`self.K2_GetActorLocation` (`self.Target`)) (0.0 0.0 200.0)) true)))

(event `self.Cube.OnComponentHit`
  (params (HitComponent :type "PrimitiveComponent Object Reference") (OtherActor :type "Actor Object Reference") (OtherComp :type "PrimitiveComponent Object Reference") (NormalImpulse :type "Vector Structure") (Hit :type "HitResult Structure (by ref)"))
  (cast `/Game/DamageSystem/Enemy/BP_Enemy` OtherActor
    (:`then`
      _)
    (:`CastFailed`
      (cast `/Game/DamageSystem/Enemy/BP_Enemy2` OtherActor
        (:`then`
          _)
        (:`CastFailed`
          (cast `/Game/DamageSystem/Drone/BP_DroneBase` OtherActor)))))
  (`PrimitiveComponent.AddImpulse` (`self.Cube`) (`KismetMathLibrary.MakeVector` 0.0 0.0 -200.0) "None" true)
  (`GameplayStatics.PlaySoundAtLocation` "/Game/Sounds/MetalHit_Cue.MetalHit_Cue" (0.0 0.0 0.0) (struct) 1.0 1.0 0.0 null null null null)
  (`GameplayStatics.SpawnEmitterAtLocation` "/Game/StarterContent/Particles/P_Sparks2.P_Sparks2")
  (`PrimitiveComponent.SetCollisionResponseToChannel` (`self.Cube`) "ECC_Pawn" "ECR_Ignore")
  (message `/Game/DamageSystem/BPI_Damageable.TakeDamage` OtherActor (make `/Game/DamageSystem/S_DamageInfo` 50.0 "NewEnumerator2" "NewEnumerator1"))
  (`KismetSystemLibrary.Delay` 2.5)
  (`self.K2_DestroyActor`))

(fn `UserConstructionScript`)