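; Base enemy drone that chases the player and fires projectile bursts.
; BeginPlay sets up the DroneAI_Controller blackboard and health bar widget, and Tick copies AIState to the blackboard.
; ChasePlayer holds attack distance, strafing on a self-restarting flip-flop timer and triggering random-length bursts aimed at the player's spine socket.
; BPCDamageSystem handles health, and its death event switches the mesh to physics before delayed destruction.
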(event `ChaseStrafe`
  (bind _isa (`/Engine/EditorBlueprintResources/StandardMacros.FlipFlop`)
    (:`A`
      _)
    (:`B`
      _))
  (set `self.ChaseStrafeRight` _isa)
  (`KismetSystemLibrary.K2_SetTimerDelegate` (delegate `ChaseStrafe`) 1.0))

(event `self.ReceiveTick`
  (params (DeltaSeconds :type "Float (single-precision)"))
  (`|ExecutionSequence`
    (:`then_0`
      (`BlackboardComponent.SetValueAsEnum` (`self.Blackboard Component Ref`) "DroneState" (`self.AIState`)))))

(event `FireEffects`
  (bind (_returnvalue_location _returnvalue_rotation) (`KismetMathLibrary.BreakTransform` (`SceneComponent.K2_GetComponentToWorld` (`self.Muzzle`))))
  (`|ExecutionSequence`
    (:`then_0`
      (`GameplayStatics.SpawnEmitterAtLocation` "/Game/StarterContent/Particles/P_Explosion.P_Explosion" _returnvalue_location _returnvalue_rotation)
      (`GameplayStatics.PlaySoundAtLocation` "/Game/StarterContent/Audio/Explosion01.Explosion01" _returnvalue_location (struct) 1.0 1.0 0.0 null null null null))
    (:`then_1`
      (`|SpawnActorFromClass` (`self.ProjectileActor`) (`SceneComponent.K2_GetComponentToWorld` (`self.Muzzle`)) "AlwaysSpawn" "MultiplyWithRoot" null null))))

(event `self.ReceiveBeginPlay`
  (`|ExecutionSequence`
    (:`then_0`
      (bind _asdrone_ai_controller (cast `/Game/DamageSystem/Drone/AIController/DroneAI_Controller` (`self.GetController`)))
      (bind _output_get (set `self.Drone AI Controller Ref` _asdrone_ai_controller))
      (bind _blackboardcomponent (`AIController.UseBlackboard` _output_get "/Game/DamageSystem/Drone/AIController/BB_DroneAI.BB_DroneAI"))
      (bind _output_get_2 (set `self.Blackboard Component Ref` _blackboardcomponent))
      (`BlackboardComponent.SetValueAsObject` _output_get_2 "DroneActor" self))
    (:`then_1`
      (set `self.StartLocation` (`self.K2_GetActorLocation`)))
    (:`then_2`
      (bind _asbp_player (cast `/Game/DamageSystem/Player/BP_Player` (`GameplayStatics.GetPlayerCharacter` 0)))
      (set `self.As BP Player` _asbp_player))
    (:`then_3`
      (`self.ChaseStrafe`))
    (:`then_4`
      (bind _returnvalue (`|CreateWidget` "/Game/DamageSystem/W_HealthBar.W_HealthBar_C" null self))
      (`WidgetComponent.SetWidget` (`self.Widget`) _returnvalue))))

(event `CheckAndFire`
  (`/Game/Blueprints/Macros/Macro.ForLoopWithDelay` 1 (`KismetMathLibrary.RandomIntegerInRange` 4 (`self.BurstFireMax`)) (`self.WeaponRecoverTime`)
    (:`LoopBody`
      (`self.FindLookAtPlayer`)
      (if (`self.IsDead?`)
        _
        (elif (not (`/Game/DamageSystem/Player/BP_Player.PlayerDead` (`self.As BP Player`)))
          (set `self.IsFiring` true)
          (`self.FireEffects`))))
    (:`Completed`
      (`KismetSystemLibrary.Delay` (`KismetMathLibrary.RandomFloatInRange` 1.0 3.0))
      (set `self.IsFiring` false))))

(event `Death`
  (`PrimitiveComponent.SetSimulatePhysics` (`self.Mesh`) true)
  (set `self.isDead?` true)
  (`PrimitiveComponent.SetCollisionEnabled` (`self.Mesh`) "QueryAndPhysics")
  (`PrimitiveComponent.SetCollisionResponseToChannel` (`self.Mesh`) "ECC_GameTraceChannel1" "ECR_Ignore")
  (`CharacterMovementComponent.DisableMovement` (`self.CharacterMovement`))
  (`ActorComponent.K2_DestroyComponent` (`self.CapsuleComponent`))
  (`KismetSystemLibrary.Delay` 10.0)
  (`self.K2_DestroyActor`))

(event `DamageResponse`
  (params (DamageResponse :type "/Game/DamageSystem/E_DamageResponse Enum" :default "NewEnumerator0"))
  (`KismetSystemLibrary.PrintString` (`|GetEnumeratorNameAsString` DamageResponse)))

(fn `ChasePlayer`
  (returns (Return :type Boolean))
  (bind (_returnvalue_x _returnvalue_y _returnvalue_z) (`KismetMathLibrary.BreakVector` (`self.K2_GetActorLocation`)))
  (bind (_returnvalue_x_2 _returnvalue_y_2) (`KismetMathLibrary.BreakVector` (`self.K2_GetActorLocation` (`self.As BP Player`))))
  (bind (_returnvalue_roll _returnvalue_pitch _returnvalue_yaw) (`KismetMathLibrary.BreakRotator` (`KismetMathLibrary.FindLookAtRotation` (`self.K2_GetActorLocation`) (`KismetMathLibrary.MakeVector` _returnvalue_x_2 _returnvalue_y_2 _returnvalue_z))))
  (bind _returnvalue (`KismetMathLibrary.Conv_RotatorToVector` (`KismetMathLibrary.MakeRotator` 0.0 0.0 _returnvalue_yaw)))
  (switch `/Game/DamageSystem/Drone/Data/Chase_States` (`self.ChaseStates`)
    (:`NewEnumerator0`
      (if (> (`self.GetDistanceTo` (`self.As BP Player`)) (`self.AttackDistance`))
        (`self.AddMovementInput` _returnvalue)
        (`self.K2_SetActorRotation` (`KismetMathLibrary.RLerp` (`self.K2_GetActorRotation`) (`KismetMathLibrary.MakeRotator` 0.0 0.0 _returnvalue_yaw) 0.1 true) :!label _label)
        (return false)
        (elif (< (`self.GetDistanceTo` (`self.As BP Player`)) (- (`self.AttackDistance`) 100.0))
          (`self.AddMovementInput` _returnvalue -1.0)
          (goto _label)
          (else
            (`self.AddMovementInput` (`KismetMathLibrary.GetRightVector` (`KismetMathLibrary.FindLookAtRotation` (`self.K2_GetActorLocation`) (`self.K2_GetActorLocation` (`self.As BP Player`)))) (`KismetMathLibrary.SelectFloat` -0.5 0.5 (`self.ChaseStrafeRight`)))
            (if (`self.IsFiring`)
              (goto _label)
              (else
                (`self.CheckAndFire`)))))))))

(fn `FindLookAtPlayer`
  (`SceneComponent.K2_SetWorldRotation` (`self.Muzzle`) (`KismetMathLibrary.FindLookAtRotation` (`SceneComponent.K2_GetComponentLocation` (`self.Muzzle`)) (`SceneComponent.GetSocketLocation` (`Character.Mesh` (`self.As BP Player`)) "spine_02")) false false))

(fn `GetCurrentHealth`
  (returns (Health :type "Float (double-precision)"))
  (return (`/Game/DamageSystem/BPC_DamageSystem.Health` (`self.BPC_DamageSystem`))))

(fn `GetMaxHealth`
  (returns (MaxHealth :type "Float (double-precision)"))
  (return (`/Game/DamageSystem/BPC_DamageSystem.MaxHealth` (`self.BPC_DamageSystem`))))

(fn `Heal`
  (params (Heal :type "Float (double-precision)"))
  (returns (NewHealth :type "Float (double-precision)"))
  (bind _newhealth (`/Game/DamageSystem/BPC_DamageSystem.Heal` (`self.BPC_DamageSystem`) Heal))
  (return _newhealth))

(fn `TakeDamage`
  (params (DamageInfo :type "/Game/DamageSystem/S_DamageInfo Structure"))
  (returns (WasDamaged :type Boolean))
  (bind _wasdamaged (`/Game/DamageSystem/BPC_DamageSystem.TakeDamage` (`self.BPC_DamageSystem`) DamageInfo))
  (return _wasdamaged))

(fn `UserConstructionScript`
  (bind _bpc_damagesystem (`self.BPC_DamageSystem`))
  (add `/Game/DamageSystem/BPC_DamageSystem.OnDeath` _bpc_damagesystem (`|CreateDelegate` :!event `Death`))
  (add `/Game/DamageSystem/BPC_DamageSystem.OnDamageResponse` _bpc_damagesystem (`|CreateDelegate` :!event `DamageResponse`)))