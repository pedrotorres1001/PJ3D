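; BP_DroneSpawner is an actor that spawns queued drone classes one at a time at its own transform.
; A looping one-second timer calls Spawner, which spawns the first class in DroneQueue and removes it.
; AddDroneToQueue appends a class and also spawns immediately if its Sphere already overlaps a BP_Drone_01.
; OnEnemyDefeated forwards the defeat notification to BP_ThirdPersonGameMode.
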(event `self.ReceiveBeginPlay`
  (`KismetSystemLibrary.K2_SetTimerDelegate` (delegate `TryToSpawn`) 1.0 true))

(event `TryToSpawn`
  (`self.Spawner`))

(event `OnEnemyDefeated`
  (bind _asbp_third_person_game_mode (cast `/Game/ThirdPerson/Blueprints/BP_ThirdPersonGameMode` (`GameplayStatics.GetGameMode`)))
  (`/Game/ThirdPerson/Blueprints/BP_ThirdPersonGameMode.OnEnemyDefeated` _asbp_third_person_game_mode))

(fn `AddDroneToQueue`
  (params (DroneClass :type "/Game/DamageSystem/Drone/BP_DroneBase Class Reference"))
  (`KismetArrayLibrary.Array_Add` (`self.DroneQueue`) DroneClass)
  (if (`KismetArrayLibrary.Array_IsValidIndex` (`PrimitiveComponent.GetOverlappingActors` (`self.Sphere`) "/Game/DamageSystem/Drone/BP_Drone_01.BP_Drone_01_C"))
    (`self.Spawner`)))

(fn `Spawner`
  (returns (Success :type Boolean))
  (if (`KismetArrayLibrary.Array_IsValidIndex` (`self.DroneQueue`))
    (`|SpawnActorFromClass` (`|GetArrayItem` (`self.DroneQueue`)) (`self.GetTransform`) "AdjustIfPossibleButAlwaysSpawn" "MultiplyWithRoot" null null)
    (`KismetArrayLibrary.Array_Remove` (`self.DroneQueue`))
    (return true)))

(fn `UserConstructionScript`)