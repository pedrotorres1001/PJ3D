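; BP_PuzzleGame is a collection puzzle that swings a door open once enough items have been collected.
; CollectItem increments the item count and tells BP_ThirdPersonGameMode to start a new wave.
; A separate OpenDoorCheck event prints the count and, at the maximum, fires OpenDoor through a DoOnce.
; OpenDoor plays a timeline that lerps the door's relative yaw to its open angle.
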(event `Open Door`
  ; Open Door Animation
  (bind (_direction _door_rotation) (`Timeline|Open Door Anim`)
    (:`Update`
      (`SceneComponent.K2_SetRelativeRotation` (`self.Door`) (`KismetMathLibrary.MakeRotator` 0.0 0.0 (`KismetMathLibrary.Lerp` 0.0 120.0 _door_rotation)) false false))))

(event `Collect Item`
  ; Collect Item Function
  (`/Engine/EditorBlueprintResources/StandardMacros.IncrementInt` (`self.CurrentItemsCollected`)
    (:`  `
      (bind _asbp_third_person_game_mode (cast `/Game/ThirdPerson/Blueprints/BP_ThirdPersonGameMode` (`GameplayStatics.GetGameMode`)))
      (`/Game/ThirdPerson/Blueprints/BP_ThirdPersonGameMode.NewWave` _asbp_third_person_game_mode))))

(event `Open Door Check`
  (bind _currentitemscollected (`self.CurrentItemsCollected`))
  (`KismetSystemLibrary.PrintString` (`KismetStringLibrary.Conv_IntToString` _currentitemscollected))
  (if (>= _currentitemscollected (`self.MaxItemsCollected`))
    (`/Engine/EditorBlueprintResources/StandardMacros.DoOnce` false
      (:`Completed`
        (`self.Open Door`)))))

(fn `UserConstructionScript`)