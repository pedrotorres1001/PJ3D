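; BP_Enemy_Test is a test enemy Character that chases the player and attacks in melee.
; From BeginPlay it uses AIMoveTo to reach the player, plays a montage whose notify triggers a sphere trace to apply damage, then resumes chasing.
; Damage reduces HP and knocks it back; at zero HP it ragdolls and is destroyed after a delay.
; A looping random-wander event exists but is not called here.
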(event `self.ReceiveBeginPlay`
  (`self.Chase Player`))

(event `Chase Player`
  (bind _attacktracepos (`self.AttackTracePos`))
  (bind _returnvalue (`SceneComponent.K2_GetComponentLocation` _attacktracepos))
  ;[1 1 1] Chase Player / AI Attack
  (`|AIMoveTo` self (0.0 0.0 0.0) (`GameplayStatics.GetPlayerCharacter` 0)
    (:`OnSuccess`
      (if (`self.AI Can Attack`)
        (`|PlayMontage` (`self.Mesh`)
          (:`then`
            (set `self.AI Can Attack` false))
          (:`OnCompleted`
            (set `self.AI Can Attack` true)
            (`self.Chase Player`))
          (:`OnNotifyBegin`
            (bind (_outhit _returnvalue_2) (`KismetSystemLibrary.SphereTraceSingleForObjects` _returnvalue (+ _returnvalue (* (`SceneComponent.GetForwardVector` _attacktracepos) 100.0)) 25.0 (`|MakeArray` "ObjectTypeQuery3" :!type "EObjectTypeQuery Enum")))
            (if _returnvalue_2
              (`GameplayStatics.ApplyDamage` (`.HitActor` (`GameplayStatics.BreakHitResult` _outhit)) 10.0))))))))

(event `Wonder`
  ;[1 1 1] Wonder
  (`|AIMoveTo` self (`NavigationSystemV1.K2_GetRandomReachablePointInRadius` (`self.K2_GetActorLocation`) 500.0 null null) null
    (:`OnSuccess`
      (`KismetSystemLibrary.Delay` 1.0)
      (`self.Wonder`))))

(event `self.ReceiveAnyDamage`
  (params (Damage :type "Float (single-precision)") (DamageType :type "DamageType Object Reference") (InstigatedBy :type "Controller Object Reference") (DamageCauser :type "Actor Object Reference"))
  ;[1 1 1] Damage
  (set `self.HP` (- (`self.HP`) Damage))
  (if (<= (`self.HP`) 0.0)
    (`PrimitiveComponent.SetSimulatePhysics` (`self.Mesh`) true)
    (set `self.AI Can Attack` false)
    (`CharacterMovementComponent.DisableMovement` (`self.CharacterMovement`))
    (`ActorComponent.K2_DestroyComponent` (`self.CapsuleComponent`))
    (`KismetSystemLibrary.Delay` 2.0)
    (`self.K2_DestroyActor`)
    (else
      (`self.LaunchCharacter` (+ (* (`self.GetActorForwardVector`) -500.0) (* (`self.GetActorUpVector`) 100.0))))))

(fn `UserConstructionScript`)