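; BP_OrbManager places the orbs that feed the snake boss in the Boss_Snake encounter.
; On BeginPlay it caches the player and snake boss, then spawns a BP_Orb at the player's location, snapped to the grid through BP_GridManager's coordinate conversions.
; Its OrbEaten event grows the snake and spawns the next orb at the player's current cell.
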(event `self.ReceiveBeginPlay`
  (bind _asbp_player (cast `/Game/DamageSystem/Player/BP_Player` (`GameplayStatics.GetPlayerCharacter` 0)))
  (set `self.BP_PlayerCharacter` _asbp_player)
  (bind _outactors (`GameplayStatics.GetAllActorsOfClass` "/Game/DamageSystem/Boss_Snake/BP_SnakeBoss.BP_SnakeBoss_C"))
  (set `self.BP_SnakeBoss` (`|GetArrayItem` _outactors))
  (`self.SpawnOrbAtPlayerLocation`))

(event `SpawnOrbAtPlayerLocation`
  (bind _outactors (`GameplayStatics.GetAllActorsOfClass` "/Game/DamageSystem/Boss_Snake/Grid/BP_GridManager.BP_GridManager_C"))
  (bind _output (`|GetArrayItem` _outactors))
  (bind (_gridx _gridy) (`/Game/DamageSystem/Boss_Snake/Grid/BP_GridManager.WorldLocationToGridCoordinates` _output (`self.K2_GetActorLocation` (`self.BP_PlayerCharacter`))))
  (bind _output_get (set `self.CurrentOrbLocationGrid` (`KismetMathLibrary.MakeVector2D` (`KismetMathLibrary.Conv_IntToDouble` _gridx) (`KismetMathLibrary.Conv_IntToDouble` _gridy))))
  (`KismetSystemLibrary.PrintString` (`KismetStringLibrary.Conv_Vector2dToString` _output_get))
  (bind _worldlocation (`/Game/DamageSystem/Boss_Snake/Grid/BP_GridManager.GridCoordinatesToWorldLocation` _output _gridx _gridy))
  (`|SpawnActorFromClass` "/Game/DamageSystem/Boss_Snake/BP_Orb.BP_Orb_C" (`KismetMathLibrary.Conv_VectorToTransform` _worldlocation) "AlwaysSpawn" "MultiplyWithRoot" null null))

(event `OrbEaten`
  (`/Game/DamageSystem/Boss_Snake/BP_SnakeBoss.GrowSnake` (`self.BP_SnakeBoss`))
  (`self.SpawnOrbAtPlayerLocation`))

(fn `UserConstructionScript`)