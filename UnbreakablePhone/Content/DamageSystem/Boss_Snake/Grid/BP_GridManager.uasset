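; Grid manager actor in the Boss_Snake folder that defines a 2D cell grid anchored at its own location.
; Helper functions convert world locations to clamped cell coordinates and cell coordinates back to world-space cell centres.
; On BeginPlay it sets the origin and draws long-lived debug boxes over every cell.
; The validity check uses strict comparisons, so border cells count as invalid.
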(event `self.ReceiveBeginPlay`
  (bind _returnvalue (/ (`self.GridCellSize`) 2.0))
  (set `self.GridOrigin` (`self.K2_GetActorLocation`))
  (for _index (range (`self.GridWitdhInCells`))
    (for _index_2 (range (`self.GridHeightInCells`))
      (bind _worldlocation (`self.GridCoordinatesToWorldLocation` _index _index_2))
      (`KismetSystemLibrary.DrawDebugBox` _worldlocation (`KismetMathLibrary.MakeVector` _returnvalue _returnvalue 1000.0) (struct :`R` 1.0 :`B` 0.08839 :`A` 1.0) (struct) 9998.0))))

(fn `GridCoordinatesToWorldLocation`
  (params (InGridX :type Integer) (InGridY :type Integer))
  (returns (WorldLocation :type "Vector Structure"))
  (bind _gridcellsize (`self.GridCellSize`))
  (bind _returnvalue (/ _gridcellsize 2.0))
  (return (+ (`KismetMathLibrary.MakeVector` (+ (* (`KismetMathLibrary.Clamp` InGridX 0 (- (`self.GridWitdhInCells`) 1)) _gridcellsize) _returnvalue) (+ (* (`KismetMathLibrary.Clamp` InGridY 0 (- (`self.GridHeightInCells`) 1)) _gridcellsize) _returnvalue)) (`self.GridOrigin`))))

(fn `IsValidGridCoordinate`
  (params (InGridX :type Integer) (InGridY :type Integer))
  (returns (NewParam :type Boolean))
  (return (and (and (> InGridX 0) (< InGridX (- (`self.GridWitdhInCells`) 1))) (and (> InGridY 0) (< InGridY (- (`self.GridHeightInCells`) 1))))))

(fn `UserConstructionScript`)

(fn `WorldLocationToGridCoordinates`
  (params (InWorldLocaction :type "Vector Structure"))
  (returns (GridX :type Integer) (GridY :type Integer))
  (bind _gridcellsize (`self.GridCellSize`))
  (return (`KismetMathLibrary.Clamp` (`KismetMathLibrary.FFloor` (/ (.x (- InWorldLocaction (`self.GridOrigin`))) _gridcellsize)) 0 (- (`self.GridWitdhInCells`) 1)) (`KismetMathLibrary.Clamp` (`KismetMathLibrary.FFloor` (/ (.y (- InWorldLocaction (`self.GridOrigin`))) _gridcellsize)) 0 (- (`self.GridHeightInCells`) 1))))