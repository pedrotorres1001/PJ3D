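; BP_Text is a single-use collectable that opens a text screen when the player interacts with it.
; A sphere overlap with BP_Player sets the proximity flags and shows or hides its widget component; both begin and end overlap enable input on the actor.
; When the player is near, IA_Interact pauses the game, shows the mouse cursor, adds WBP_Text to the viewport and destroys the actor.
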(event `EnhancedInput|/Game/ThirdPerson/Input/Actions/IA_Interact`
  (params (ActionValue :type Boolean) (ElapsedSeconds :type "Float (double-precision)") (TriggeredSeconds :type "Float (double-precision)") (InputAction :type "InputAction Object Reference" :default "/Game/ThirdPerson/Input/Actions/IA_Interact.IA_Interact"))
  (:`Triggered`
    (if (`self.isPlayerNear`)
      (`GameplayStatics.SetGamePaused` true)
      (set `PlayerController.bShowMouseCursor` true (`GameplayStatics.GetPlayerController` 0))
      (bind _returnvalue (`|CreateWidget` "/Game/DamageSystem/Collectables/WBP/WBP_Text.WBP_Text_C"))
      (bind _output_get (set `self.OpenText` _returnvalue))
      (`UserWidget.AddToViewport` _output_get 0)
      (`self.K2_DestroyActor`))))

(event `self.Sphere.OnComponentBeginOverlap`
  (params (OverlappedComponent :type "PrimitiveComponent Object Reference") (OtherActor :type "Actor Object Reference") (OtherComp :type "PrimitiveComponent Object Reference") (OtherBodyIndex :type Integer) (bFromSweep :type Boolean) (SweepResult :type "HitResult Structure (by ref)"))
  (cast `/Game/DamageSystem/Player/BP_Player` OtherActor)
  (`self.EnableInput` (`GameplayStatics.GetPlayerController` 0))
  (`SceneComponent.SetVisibility` (`self.Widget`) true false)
  (set `self.isPlayerNear` true)
  (set `self.HasBeenActivated` true))

(event `self.Sphere.OnComponentEndOverlap`
  (params (OverlappedComponent :type "PrimitiveComponent Object Reference") (OtherActor :type "Actor Object Reference") (OtherComp :type "PrimitiveComponent Object Reference") (OtherBodyIndex :type Integer))
  (cast `/Game/DamageSystem/Player/BP_Player` OtherActor)
  (`self.EnableInput` (`GameplayStatics.GetPlayerController` 0))
  (`SceneComponent.SetVisibility` (`self.Widget`) false false)
  (set `self.isPlayerNear` false)
  (set `self.HasBeenActivated` false))

(fn `UserConstructionScript`)