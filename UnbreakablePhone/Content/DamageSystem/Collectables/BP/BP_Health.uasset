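; BP_Health is a collectable health pickup that fully restores the player's health.
; Its Cube bobs vertically each tick on a sine of game time around its starting height.
; When a BP_Player overlaps the Sphere, it sets the damage component's Health to MaxHealth, plays a sound and destroys itself.
; An unconnected leftover graph would resize a widget's draw size by distance to the player, but never runs.
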(event `self.ReceiveBeginPlay`
  (bind (_relativelocation_x _relativelocation_y _relativelocation_z) (`KismetMathLibrary.BreakVector` (`SceneComponent.RelativeLocation` (`self.Cube`))))
  (set `self.BaseZ` _relativelocation_z))

(event `self.ReceiveTick`
  (params (DeltaSeconds :type "Float (single-precision)"))
  (bind _cube (`self.Cube`))
  (bind (_relativelocation_x _relativelocation_y _relativelocation_z) (`KismetMathLibrary.BreakVector` (`SceneComponent.RelativeLocation` _cube)))
  (`SceneComponent.K2_SetRelativeLocation` _cube (`KismetMathLibrary.MakeVector` _relativelocation_x _relativelocation_y (+ (`self.BaseZ`) (* (`self.BobAmplitude`) (`KismetMathLibrary.Sin` (* (`self.BobSpeed`) (`KismetSystemLibrary.GetGameTimeInSeconds`)))))) false false))

(event `self.Sphere.OnComponentBeginOverlap`
  (params (OverlappedComponent :type "PrimitiveComponent Object Reference") (OtherActor :type "Actor Object Reference") (OtherComp :type "PrimitiveComponent Object Reference") (OtherBodyIndex :type Integer) (bFromSweep :type Boolean) (SweepResult :type "HitResult Structure (by ref)"))
  (bind _asbp_player (cast `/Game/DamageSystem/Player/BP_Player` OtherActor))
  (`self.EnableInput` (`GameplayStatics.GetPlayerController` 0))
  (bind _bpc_damagesystem (`/Game/DamageSystem/Player/BP_Player.BPC_DamageSystem` _asbp_player))
  (set `/Game/DamageSystem/BPC_DamageSystem.Health` (`/Game/DamageSystem/BPC_DamageSystem.MaxHealth` _bpc_damagesystem) _bpc_damagesystem)
  (`GameplayStatics.PlaySound2D` "/Game/Sounds/powerup.powerup" 1.0 1.0 0.0 null null)
  (`self.K2_DestroyActor`))

(fn `UserConstructionScript`)