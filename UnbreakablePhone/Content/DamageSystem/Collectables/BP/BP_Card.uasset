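; Collectible key card that the player picks up with E, flagging PickedUpKey on BP_Player.
; Box overlap shows a prompt widget and opens a gate for the key press.
; Pickup flashes a collected widget, then destroys the card and reveals the player HUD's grenade panel.
; An arrow widget bobs on a sine wave, faces the camera and hides while the player is inside ArrowSphere.
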(event `self.ReceiveBeginPlay`
  (bind (_relativelocation_x _relativelocation_y _relativelocation_z) (`KismetMathLibrary.BreakVector` (`SceneComponent.RelativeLocation` (`self.ArrowWidget`))))
  (set `self.BaseZ` _relativelocation_z))

(event `self.ReceiveTick`
  (params (DeltaSeconds :type "Float (single-precision)"))
  (bind _arrowwidget (`self.ArrowWidget`))
  (bind (_relativelocation_x _relativelocation_y _relativelocation_z) (`KismetMathLibrary.BreakVector` (`SceneComponent.RelativeLocation` (`self.ArrowWidget`))))
  (`SceneComponent.K2_SetRelativeLocation` (`self.ArrowWidget`) (`KismetMathLibrary.MakeVector` _relativelocation_x _relativelocation_y (+ (`self.BaseZ`) (* (`self.BobAmplitude`) (`KismetMathLibrary.Sin` (* (`self.BobSpeed`) (`KismetSystemLibrary.GetGameTimeInSeconds`)))))) false false)
  (`SceneComponent.K2_SetWorldRotation` _arrowwidget (`KismetMathLibrary.FindLookAtRotation` (`SceneComponent.K2_GetComponentLocation` _arrowwidget) (`PlayerCameraManager.GetCameraLocation` (`GameplayStatics.GetPlayerCameraManager` 0))) false false))

(event `Key|E`
  (params (Key :type "Key Structure"))
  (:`Pressed`
    (`/Engine/EditorBlueprintResources/StandardMacros.Gate` true :!label _label
      (:`Exit`
        (set `/Game/DamageSystem/Player/BP_Player.PickedUpKey` true (stale `self.Box.OnComponentBeginOverlap` _asbp_player))
        (bind _returnvalue (`|CreateWidget` "/Game/DamageSystem/Collectables/WBP/WBP_CardCollected.WBP_CardCollected_C"))
        (`UserWidget.AddToViewport` _returnvalue 0)
        (`KismetSystemLibrary.Delay` 1.5)
        (`Widget.RemoveFromParent` _returnvalue)
        (`self.K2_DestroyActor`)
        (bind _asbp_player (cast `/Game/DamageSystem/Player/BP_Player` (`GameplayStatics.GetPlayerPawn` 0)))
        (set `Widget.Visibility` "Visible" (`/Game/DamageSystem/Player/UI_PlayerHealthBar.GrenadePanel` (`/Game/DamageSystem/Player/BP_Player.UI_HealthBar` _asbp_player)))))))

(event `self.Box.OnComponentBeginOverlap`
  (params (OverlappedComponent :type "PrimitiveComponent Object Reference") (OtherActor :type "Actor Object Reference") (OtherComp :type "PrimitiveComponent Object Reference") (OtherBodyIndex :type Integer) (bFromSweep :type Boolean) (SweepResult :type "HitResult Structure (by ref)"))
  (bind _asbp_player (cast `/Game/DamageSystem/Player/BP_Player` OtherActor))
  (`SceneComponent.SetVisibility` (`self.Widget`) true false)
  (`self.EnableInput` (`GameplayStatics.GetPlayerController` 0))
  (goto _label :!via `Open`))

(event `self.Box.OnComponentEndOverlap`
  (params (OverlappedComponent :type "PrimitiveComponent Object Reference") (OtherActor :type "Actor Object Reference") (OtherComp :type "PrimitiveComponent Object Reference") (OtherBodyIndex :type Integer))
  (cast `/Game/DamageSystem/Player/BP_Player` OtherActor)
  (`SceneComponent.SetVisibility` (`self.Widget`) false false)
  (`self.EnableInput` (`GameplayStatics.GetPlayerController` 0))
  (goto _label :!via `Close`))

(event `self.ArrowSphere.OnComponentBeginOverlap`
  (params (OverlappedComponent :type "PrimitiveComponent Object Reference") (OtherActor :type "Actor Object Reference") (OtherComp :type "PrimitiveComponent Object Reference") (OtherBodyIndex :type Integer) (bFromSweep :type Boolean) (SweepResult :type "HitResult Structure (by ref)"))
  (cast `/Game/DamageSystem/Player/BP_Player` OtherActor)
  (`SceneComponent.SetVisibility` (`self.ArrowWidget`) false false))

(event `self.ArrowSphere.OnComponentEndOverlap`
  (params (OverlappedComponent :type "PrimitiveComponent Object Reference") (OtherActor :type "Actor Object Reference") (OtherComp :type "PrimitiveComponent Object Reference") (OtherBodyIndex :type Integer))
  (cast `/Game/DamageSystem/Player/BP_Player` OtherActor)
  (`SceneComponent.SetVisibility` (`self.ArrowWidget`) true false))

(fn `UserConstructionScript`)