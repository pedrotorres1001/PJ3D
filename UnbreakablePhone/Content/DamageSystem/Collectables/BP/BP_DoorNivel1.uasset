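; BP_DoorNivel1 is a one-way door that the player opens by pressing E inside its trigger box.
; Overlap by BP_Player shows a prompt widget, enables input and opens a gate, all reversed on exit.
; E hides the prompt and, if the Somethign flag is set, passes the gate to set DoorOpened, play a sound and start a timeline.
; The timeline slides the door along relative X by a fixed step per update.
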(event `self.Box.OnComponentBeginOverlap`
  (params (OverlappedComponent :type "PrimitiveComponent Object Reference") (OtherActor :type "Actor Object Reference") (OtherComp :type "PrimitiveComponent Object Reference") (OtherBodyIndex :type Integer) (bFromSweep :type Boolean) (SweepResult :type "HitResult Structure (by ref)"))
  (bind (_relativelocation_x _relativelocation_y _relativelocation_z) (`KismetMathLibrary.BreakVector` (`SceneComponent.RelativeLocation` (`self.door`))))
  (cast `/Game/DamageSystem/Player/BP_Player` OtherActor)
  (if (not (`self.DoorOpened`))
    (`SceneComponent.SetVisibility` (`self.Widget`) true false)
    (`self.EnableInput` (`GameplayStatics.GetPlayerController` 0))
    (goto _label :!via `Open`)))

(event `self.Box.OnComponentEndOverlap`
  (params (OverlappedComponent :type "PrimitiveComponent Object Reference") (OtherActor :type "Actor Object Reference") (OtherComp :type "PrimitiveComponent Object Reference") (OtherBodyIndex :type Integer))
  (bind (_relativelocation_x _relativelocation_y _relativelocation_z) (`KismetMathLibrary.BreakVector` (`SceneComponent.RelativeLocation` (`self.door`))))
  (cast `/Game/DamageSystem/Player/BP_Player` OtherActor)
  (`SceneComponent.SetVisibility` (`self.Widget`) false false)
  (`self.DisableInput` (`GameplayStatics.GetPlayerController` 0))
  (goto _label :!via `Close`))

(event `Key|E`
  (params (Key :type "Key Structure"))
  (bind (_relativelocation_x _relativelocation_y _relativelocation_z) (`KismetMathLibrary.BreakVector` (`SceneComponent.RelativeLocation` (`self.door`))))
  (:`Pressed`
    (`SceneComponent.SetVisibility` (`self.Widget`) false false)
    (if (`self.somethign`)
      (`/Engine/EditorBlueprintResources/StandardMacros.Gate` true :!label _label
        (:`Exit`
          (`/Engine/EditorBlueprintResources/StandardMacros.FlipFlop`
            (:`A`
              (if (not (`self.DoorOpened`))
                (set `self.DoorOpened` true)
                (`GameplayStatics.PlaySoundAtLocation` "/Game/Sounds/door.door" (`SceneComponent.K2_GetComponentLocation` (`self.door`)) (struct) 1.0 1.0 0.0 null null null null)
                (`Timeline|OpenDoor`
                  (:`Update`
                    (`SceneComponent.K2_SetRelativeLocation` (`self.door`) (`KismetMathLibrary.MakeVector` (+ _relativelocation_x 1.5) _relativelocation_y _relativelocation_z) false false)))))))))))

(fn `UserConstructionScript`)