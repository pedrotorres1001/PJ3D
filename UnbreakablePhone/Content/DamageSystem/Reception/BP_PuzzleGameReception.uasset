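; BP_PuzzleGameReception is a door actor that exits to the "Principal" level once all collectables are gathered.
; Its Trigger enables input while BP_Player overlaps it and disables it on exit.
; Pressing E checks that the game mode's CollectablesLeft is zero, then plays a timeline that swings the door open on yaw.
; The level open runs from the timeline's Update, so it fires without waiting for the swing to finish.
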(event `Key|E`
  (params (Key :type "Key Structure"))
  ; Open Door Anim
  (:`Pressed`
    (bind _asbp_third_person_game_mode (cast `/Game/ThirdPerson/Blueprints/BP_ThirdPersonGameMode` (`GameplayStatics.GetGameMode`)))
    (if (== (`/Game/ThirdPerson/Blueprints/BP_ThirdPersonGameMode.Collectables Left` _asbp_third_person_game_mode) 0)
      (bind (_direction _door_rotation) (`Timeline|Open Door Anim`)
        (:`Update`
          (`SceneComponent.K2_SetRelativeRotation` (`self.Door`) (`KismetMathLibrary.MakeRotator` 0.0 0.0 (`KismetMathLibrary.Lerp` 0.0 120.0 _door_rotation)) false false)
          (`GameplayStatics.OpenLevel` "Principal"))))))

(event `self.Trigger.OnComponentBeginOverlap`
  (params (OverlappedComponent :type "PrimitiveComponent Object Reference") (OtherActor :type "Actor Object Reference") (OtherComp :type "PrimitiveComponent Object Reference") (OtherBodyIndex :type Integer) (bFromSweep :type Boolean) (SweepResult :type "HitResult Structure (by ref)"))
  (cast `/Game/DamageSystem/Player/BP_Player` OtherActor)
  (`self.EnableInput` (`GameplayStatics.GetPlayerController` 0)))

(event `self.Trigger.OnComponentEndOverlap`
  (params (OverlappedComponent :type "PrimitiveComponent Object Reference") (OtherActor :type "Actor Object Reference") (OtherComp :type "PrimitiveComponent Object Reference") (OtherBodyIndex :type Integer))
  (cast `/Game/DamageSystem/Player/BP_Player` OtherActor)
  (`self.DisableInput` (`GameplayStatics.GetPlayerController` 0)))

(fn `UserConstructionScript`)