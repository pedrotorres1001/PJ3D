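; Tutorial controller that introduces the Ricochet, Grenade and Tetris abilities in order through prompts in the player's UIHealthBar.
; BeginPlay caches the player, shows the Ricochet prompt and spawns two BP_Enemy2 at a fixed location.
; Boolean flags make each input count once and in sequence, advancing the prompt after a short delay.
; Ricochet and Grenade steps each spawn another enemy; Tetris ends by showing all three panels.
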(event `EnhancedInput|/Game/ThirdPerson/Input/Actions/IA_Ricochet`
  (params (ActionValue :type Boolean) (ElapsedSeconds :type "Float (double-precision)") (TriggeredSeconds :type "Float (double-precision)") (InputAction :type "InputAction Object Reference" :default "/Game/ThirdPerson/Input/Actions/IA_Ricochet.IA_Ricochet"))
  (:`Triggered`
    (if (not (`self.HasRBeenPressed`))
      (set `self.HasRBeenPressed` true)
      (`KismetSystemLibrary.Delay` 2.0)
      (bind _ui_healthbar (`/Game/DamageSystem/Player/BP_Player.UI_HealthBar` (stale `self.ReceiveBeginPlay` _asbp_player)))
      (set `Widget.Visibility` "Hidden" (`/Game/DamageSystem/Player/UI_PlayerHealthBar.RicochetPanel` _ui_healthbar))
      (set `Widget.Visibility` "Hidden" (`/Game/DamageSystem/Player/UI_PlayerHealthBar.Ricochet_Text` _ui_healthbar))
      (set `Widget.Visibility` "Visible" (`/Game/DamageSystem/Player/UI_PlayerHealthBar.GrenadePanel` _ui_healthbar))
      (set `Widget.Visibility` "Visible" (`/Game/DamageSystem/Player/UI_PlayerHealthBar.Grenade_Text` _ui_healthbar))
      (`|SpawnActorFromClass` "/Game/DamageSystem/Enemy/BP_Enemy2.BP_Enemy2_C" (`KismetMathLibrary.MakeTransform` (1800.0 -600.0 100.0) (struct :`Yaw` 90.0)) "Undefined" "MultiplyWithRoot" null null))))

(event `EnhancedInput|/Game/ThirdPerson/Input/Actions/IA_Grenade`
  (params (ActionValue :type Boolean) (ElapsedSeconds :type "Float (double-precision)") (TriggeredSeconds :type "Float (double-precision)") (InputAction :type "InputAction Object Reference" :default "/Game/ThirdPerson/Input/Actions/IA_Grenade.IA_Grenade"))
  (:`Triggered`
    (if (`self.HasRBeenPressed`)
      (if (not (`self.HasGBeenPressed`))
        (set `self.HasGBeenPressed` true)
        (`KismetSystemLibrary.Delay` 2.0)
        (bind _ui_healthbar (`/Game/DamageSystem/Player/BP_Player.UI_HealthBar` (stale `self.ReceiveBeginPlay` _asbp_player)))
        (set `Widget.Visibility` "Hidden" (`/Game/DamageSystem/Player/UI_PlayerHealthBar.RicochetPanel` _ui_healthbar))
        (set `Widget.Visibility` "Hidden" (`/Game/DamageSystem/Player/UI_PlayerHealthBar.Ricochet_Text` _ui_healthbar))
        (set `Widget.Visibility` "Hidden" (`/Game/DamageSystem/Player/UI_PlayerHealthBar.GrenadePanel` _ui_healthbar))
        (set `Widget.Visibility` "Hidden" (`/Game/DamageSystem/Player/UI_PlayerHealthBar.Grenade_Text` _ui_healthbar))
        (set `Widget.Visibility` "Visible" (`/Game/DamageSystem/Player/UI_PlayerHealthBar.TetrisPanel` _ui_healthbar))
        (set `Widget.Visibility` "Visible" (`/Game/DamageSystem/Player/UI_PlayerHealthBar.Tetris_Text` _ui_healthbar))
        (`|SpawnActorFromClass` "/Game/DamageSystem/Enemy/BP_Enemy2.BP_Enemy2_C" (`KismetMathLibrary.MakeTransform` (1800.0 -600.0 100.0) (struct :`Yaw` 90.0)) "Undefined" "MultiplyWithRoot" null null)))))

(event `EnhancedInput|/Game/ThirdPerson/Input/Actions/IA_Tetris`
  (params (ActionValue :type Boolean) (ElapsedSeconds :type "Float (double-precision)") (TriggeredSeconds :type "Float (double-precision)") (InputAction :type "InputAction Object Reference" :default "/Game/ThirdPerson/Input/Actions/IA_Tetris.IA_Tetris"))
  (:`Triggered`
    (if (`self.HasGBeenPressed`)
      (if (not (`self.HasTBeenPressed`))
        (set `self.HasTBeenPressed` true)
        (`KismetSystemLibrary.Delay` 2.0)
        (bind _ui_healthbar (`/Game/DamageSystem/Player/BP_Player.UI_HealthBar` (stale `self.ReceiveBeginPlay` _asbp_player)))
        (set `Widget.Visibility` "Visible" (`/Game/DamageSystem/Player/UI_PlayerHealthBar.GrenadePanel` _ui_healthbar))
        (set `Widget.Visibility` "Visible" (`/Game/DamageSystem/Player/UI_PlayerHealthBar.RicochetPanel` _ui_healthbar))
        (set `Widget.Visibility` "Visible" (`/Game/DamageSystem/Player/UI_PlayerHealthBar.TetrisPanel` _ui_healthbar))
        (set `Widget.Visibility` "Hidden" (`/Game/DamageSystem/Player/UI_PlayerHealthBar.Tetris_Text` _ui_healthbar))))))

(event `self.ReceiveBeginPlay`
  (`KismetSystemLibrary.Delay` 0.01)
  (bind _asbp_player (cast `/Game/DamageSystem/Player/BP_Player` (`GameplayStatics.GetPlayerPawn` 0)))
  (bind _ui_healthbar (`/Game/DamageSystem/Player/BP_Player.UI_HealthBar` _asbp_player))
  (set `Widget.Visibility` "Hidden" (`/Game/DamageSystem/Player/UI_PlayerHealthBar.GrenadePanel` _ui_healthbar))
  (bind _ricochetpanel (`/Game/DamageSystem/Player/UI_PlayerHealthBar.RicochetPanel` _ui_healthbar))
  (set `Widget.Visibility` "Hidden" _ricochetpanel)
  (set `Widget.Visibility` "Hidden" (`/Game/DamageSystem/Player/UI_PlayerHealthBar.TetrisPanel` _ui_healthbar))
  (bind _ricochet_text (`/Game/DamageSystem/Player/UI_PlayerHealthBar.Ricochet_Text` _ui_healthbar))
  (set `Widget.Visibility` "Hidden" _ricochet_text)
  (set `Widget.Visibility` "Hidden" (`/Game/DamageSystem/Player/UI_PlayerHealthBar.Grenade_Text` _ui_healthbar))
  (set `Widget.Visibility` "Hidden" (`/Game/DamageSystem/Player/UI_PlayerHealthBar.Tetris_Text` _ui_healthbar))
  (`|SpawnActorFromClass` "/Game/DamageSystem/Enemy/BP_Enemy2.BP_Enemy2_C" (`KismetMathLibrary.MakeTransform` (1800.0 -600.0 100.0) (struct :`Yaw` 90.0)) "Undefined" "MultiplyWithRoot" null null)
  (`|SpawnActorFromClass` "/Game/DamageSystem/Enemy/BP_Enemy2.BP_Enemy2_C" (`KismetMathLibrary.MakeTransform` (1800.0 -600.0 100.0) (struct :`Yaw` 90.0)) "Undefined" "MultiplyWithRoot" null null)
  (set `Widget.Visibility` "Visible" _ricochetpanel)
  (set `Widget.Visibility` "Visible" _ricochet_text))

(fn `UserConstructionScript`)